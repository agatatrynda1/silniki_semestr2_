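; Player pawn that rolls a Sphere by physics torque and restarts the level when damaged.
; Both movement axes feed one AddTorqueInRadians node on X and Y, scaled by Multiplier and applied as acceleration change, ignoring mass.
; Any damage calls DamageLevelRestart, which fades the camera out, waits for the fade, then reopens the current level.
; Escape quits the game.
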(event Game|Damage|EventAnyDamage
  (params (Damage :type Float%20%28single-precision%29) (DamageType :type Damage%20Type%20Object%20Reference) (InstigatedBy :type Controller%20Object%20Reference) (DamageCauser :type Actor%20Object%20Reference))
  (Utilities|DamageLevelRestart))

(event Input|AxisEvents|InputAxisMoveForward/Backwards
  (params (AxisValue :type Float%20%28single-precision%29))
  (bind _multiplier (Variables|Default|GetMultiplier))
  (Class|PrimitiveComponent|AddTorqueinRadians (Variables|Default|GetSphere) (Math|Vector|MakeVector (* (stale Input|AxisEvents|InputAxisMoveLeft/Righ AxisValue) _multiplier) (* AxisValue _multiplier) 0.0) "None" true))

(event Input|AxisEvents|InputAxisMoveLeft/Righ
  (params (AxisValue :type Float%20%28single-precision%29))
  (bind _multiplier (Variables|Default|GetMultiplier))
  (Class|PrimitiveComponent|AddTorqueinRadians (Variables|Default|GetSphere) (Math|Vector|MakeVector (* AxisValue _multiplier) (* (stale Input|AxisEvents|InputAxisMoveForward/Backwards AxisValue) _multiplier) 0.0) "None" true))

(event Input|KeyboardEvents|Escape
  (params (Key :type Key%20Structure))
  (:Pressed
    (Game|QuitGame 0 "Quit")))

(fn ConstructionScript)
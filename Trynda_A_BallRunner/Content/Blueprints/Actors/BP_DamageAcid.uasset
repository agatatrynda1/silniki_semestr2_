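; BP_DamageAcid is an acid hazard actor that applies damage to the player pawn when it begins overlapping it.
; When IsMovable is set, BeginPlay caches the actor's scale and runs the ActorScale timeline to lerp it between that scale and zero.
; The timeline restarts each time it finishes, so the scale animation repeats endlessly.
; Damage fires once per overlap begin and ignores all other actors.
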(event Collision|EventActorBeginOverlap
  (params (OtherActor :type Actor%20Object%20Reference))
  (bind _returnvalue (Game|Player|GetPlayerPawn 0))
  (if (== OtherActor _returnvalue)
    (Game|Damage|ApplyDamage _returnvalue 1.0 0 0)))

(event EventBeginPlay
  (if (Variables|Default|GetIsMovable)
    (Variables|Default|SetStartScale (Transformation|GetActorScale3D))
    (bind _alphascale (Timeline|ActorScale Play)
      (:Update
        (Transformation|SetActorScale3D (Math|Vector|Lerp(Vector) (Variables|Default|GetStartScale) "0, 0, 0" _alphascale)))
      (:Finished
        (Timeline|ActorScale PlayFromStart)))))

(fn ConstructionScript)
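; BP_Cannon is an actor that fires BP_cannonball projectiles repeatedly and automatically from BeginPlay.
; Each cycle spawns a cannonball at the Arrow component's location and rotation, scaled by ProjectileScale, then plays CannonFireTimeline from the start.
; The timeline drives the Cannon component's relative Y location to animate the barrel, and its Cannon Fired event waits ProjectilePace seconds before looping back to fire again.
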(event EventBeginPlay
  (CallFunction|SpawnProjectile :!label _label)
  (bind _cannonbarrellocation (Timeline|Cannon%20Fire%20Timeline PlayFromStart)
    (:Update
      (CallFunction|SetCannonLocation _cannonbarrellocation))
    (:Cannon%20Fired
      (Utilities|FlowControl|Delay (Variables|CannonProperties|GetProjectilePace))
      (goto _label))))

(fn ConstructionScript)

(fn SpawnProjectile
  (bind _arrow (Variables|Default|GetArrow))
  (bind _returnvalue (Transformation|GetWorldTransform _arrow))
  (Game|SpawnActorfromClass "/Game/Blueprints/Actors/Projectiles/BP_cannonball.BP_cannonball_C" (Math|Transform|MakeTransform (.location _returnvalue) (.rotation _returnvalue) (Math|Conversions|ToVector(Float) (Variables|CannonProperties|GetProjectile%20Scale))) "Undefined" 0 0))

(fn SetCannonLocation
  (params (CannonBarrelY%20Location :type Float%20%28single-precision%29))
  (Transformation|SetRelativeLocation (Variables|Default|GetCannon) (Math|Vector|MakeVector 0.0 CannonBarrelY%20Location 0.0) false false))
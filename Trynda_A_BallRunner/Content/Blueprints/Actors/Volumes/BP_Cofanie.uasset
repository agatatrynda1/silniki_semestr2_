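; BP_Cofanie is a volume actor that sends the player back to a reset location while any crystals remain in the level.
; On actor overlap it filters for the player, then calls CheckAnyCrystal, which returns true only when no BP_Crystal actors exist, despite its name.
; If that check fails, the player pawn is moved to the ResetLocatin variable without sweep; otherwise the player passes unaffected.
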(event EventBeginPlay)

(event Collision|EventActorBeginOverlap
  (params (OtherActor :type Actor%20Object%20Reference))
  (Utilities|IsPlayer OtherActor
    (:IsPlayer
      (if (not (Pure|CheckAnyCrystal))
        (Transformation|SetActorLocation (Game|Player|GetPlayerPawn 0) (Variables|Default|GetResetLocatin) false false)))))

(event EventTick
  (params (DeltaSeconds :type Float%20%28single-precision%29)))

(fn ConstructionScript)

(fn CheckAnyCrystal
  (bind _outactors (Actor|GetAllActorsOfClass "/Game/Blueprints/Actors/Collectables/BP_Crystal.BP_Crystal_C"))
  (return (== (Utilities|Array|Length _outactors) 0)))
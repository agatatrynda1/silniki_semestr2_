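; Collectable crystal that spins in place and, when the player pawn overlaps it, flies into the player and disappears.
; Tick adds a fixed yaw step each frame, independent of delta time.
; On overlap it caches location, scale and light intensity, then a timeline lerps it toward the pawn's live position while shrinking it and fading its point light.
; The actor destroys itself when the timeline finishes.
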(event EventBeginPlay)

(event Collision|EventActorBeginOverlap
  (params (OtherActor :type Actor%20Object%20Reference))
  (Utilities|IsPlayer OtherActor
    (:IsPlayer
      (CallFunction|GetStartLocationScaleandIntensity)
      (bind (_direction _smoothlerpalpha _lightintensityalpha) (Timeline|TL_BlendAlpha Play)
        (:Update
          (CallFunction|MoveCrystaltoPawn _smoothlerpalpha)
          (CallFunction|ChangeCrystalScale _smoothlerpalpha)
          (CallFunction|ChangeLightIntensity _lightintensityalpha))
        (:Finished
          (Actor|DestroyActor))))))

(event EventTick
  (params (DeltaSeconds :type Float%20%28single-precision%29))
  (bind _returnvalue (Transformation|GetActorRotation))
  (Transformation|SetActorRotation (Math|Rotator|MakeRotator (.roll _returnvalue) (.pitch _returnvalue) (+ (.yaw _returnvalue) 1.0))))

(fn ConstructionScript)

(fn MoveCrystaltoPawn
  (params (Alpha :type Float%20%28single-precision%29))
  (Transformation|SetActorLocation (Math|Vector|Lerp(Vector) (Variables|Default|GetLerpStartLocation) (Transformation|GetActorLocation (Game|Player|GetPlayerPawn 0)) Alpha) false false))

(fn GetStartLocationScaleandIntensity
  (Variables|Default|SetLerpStartLocation (Transformation|GetActorLocation))
  (Variables|Default|SetLerpStartScale (Transformation|GetActorScale3D))
  (Variables|Default|SetLerpStartIntensity (Variables|/Script/Engine.LightComponentBase|GetIntensity (Variables|Default|GetPointLight))))

(fn ChangeCrystalScale
  (params (Alpha :type Float%20%28single-precision%29))
  (Transformation|SetActorScale3D (Math|Vector|Lerp(Vector) (Variables|Default|GetLerpStartScale) "0, 0, 0" Alpha)))

(fn ChangeLightIntensity
  (params (Alpha :type Float%20%28single-precision%29))
  (Rendering|Components|Light|SetIntensity (Variables|Default|GetPointLight) (Math|Float|Lerp (Variables|Default|GetLerpStartIntensity) 0.0 Alpha)))